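; BP_Pig is a destructible pig actor that dies from hard physics impacts.
; On mesh hit, a fast-moving pig spawns a dust emitter and destroys itself.
; Otherwise, hits from BP_BaseWalls pass the wall's speed to Damage, which counts hard impacts and destroys the pig when the counter reaches its limit.
; Walls moving above a higher speed threshold are destroyed as well.
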(event OnComponentHit(PigMesh)
  (params (HitComponent :type Primitive%20Component%20Object%20Reference) (OtherActor :type Actor%20Object%20Reference) (OtherComp :type Primitive%20Component%20Object%20Reference) (NormalImpulse :type Vector :default "0, 0, 0") (Hit :type Hit%20Result%20Structure%20%28by%20ref%29))
  (if (> (Math|Vector|VectorLength (Transformation|GetComponentVelocity (Variables|Default|GetPigMesh))) 2e+02)
    (Effects|SpawnEmitteratLocation "/Game/StarterContent/Particles/P_Ambient_Dust.P_Ambient_Dust" (Transformation|GetActorLocation))
    (Actor|DestroyActor)
    (else
      (bind _asbp_base_walls (Utilities|Casting|CastToBP_BaseWalls OtherActor))
      (CallFunction|Damage (Math|Vector|VectorLength (Transformation|GetComponentVelocity (Variables|/Game/Blueprints/BP_BaseWalls.BP_BaseWalls_C|GetStaticMesh _asbp_base_walls))))
      (if (> (Math|Vector|VectorLength (Transformation|GetComponentVelocity (Variables|/Game/Blueprints/BP_BaseWalls.BP_BaseWalls_C|GetStaticMesh _asbp_base_walls))) 2.5e+02)
        (Actor|DestroyActor _asbp_base_walls)))))

(event EventBeginPlay)

(event Collision|EventActorBeginOverlap
  (params (OtherActor :type Actor%20Object%20Reference)))

(event EventTick
  (params (DeltaSeconds :type Float%20%28single-precision%29)))

(fn ConstructionScript)

(fn Damage
  (params (A :type Float%20%28double-precision%29))
  (if (> A 2e+02)
    (bind _result (Math|Integer|IncrementInt (Variables|Default|GetSelection))
      (:%20%20
        (switch int _result
          (:2
            (Actor|DestroyActor)))))))
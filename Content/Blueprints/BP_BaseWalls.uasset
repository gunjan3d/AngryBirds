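; BP_BaseWalls is a destructible wall block that reacts to bird and pig collisions, Angry Birds style.
; On mesh hit, a bird's speed feeds Damage, which above a threshold randomly swaps the material to oak, destroys the wall or does nothing.
; A fast-moving wall hitting a pig spawns an explosion, destroys the pig, then destroys itself after a short delay.
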(event OnComponentHit(StaticMesh)
  (params (HitComponent :type Primitive%20Component%20Object%20Reference) (OtherActor :type Actor%20Object%20Reference) (OtherComp :type Primitive%20Component%20Object%20Reference) (NormalImpulse :type Vector :default "0, 0, 0") (Hit :type Hit%20Result%20Structure%20%28by%20ref%29))
  (bind _asbp_birds (Utilities|Casting|CastToBP_Birds OtherActor)
    (:then
      (CallFunction|Damage (Math|Vector|VectorLength (Transformation|GetComponentVelocity (Variables|/Game/Blueprints/BP_Birds.BP_Birds_C|GetBird _asbp_birds))))
      (bind _asbp_pig (Utilities|Casting|CastToBP_Pig OtherActor :!label _label))
      (Effects|SpawnEmitteratLocation "/Game/StarterContent/Particles/P_Explosion.P_Explosion" (Transformation|GetActorLocation _asbp_pig))
      (Actor|DestroyActor _asbp_pig)
      (Utilities|FlowControl|Delay 0.7)
      (Actor|DestroyActor))
    (:CastFailed
      (if (> (Math|Vector|VectorLength (Transformation|GetComponentVelocity (Variables|Default|GetStaticMesh))) 1.5e+02)
        (goto _label)))))

(fn ConstructionScript)

(fn Damage
  (params (A :type Float%20%28double-precision%29))
  (if (> A 2e+02)
    (switch int (Math|Random|RandomIntegerinRange 0 3)
      (:1
        (Rendering|Material|SetMaterial (Variables|Default|GetStaticMesh) 0 "/Game/StarterContent/Materials/M_Wood_Oak.M_Wood_Oak"))
      (:2
        (Actor|DestroyActor)))))